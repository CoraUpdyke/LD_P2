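; BP_PlayCon is a player controller that sets up input and handles pausing.
; On BeginPlay it adds the main Enhanced Input mapping context, sets game-only input and caches the gameplay HUD.
; Releasing the pause action runs a FlipFlop toggle for game pause, mouse cursor, pause widget visibility and input mode.
; Pausing also focuses the pause widget and sends the HUD an empty objective-text update.
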(event `self.ReceiveBeginPlay`
  (`EnhancedInputSubsystemInterface.AddMappingContext` (subsystem `EnhancedInputLocalPlayerSubsystem`) "/Game/Assets/BP/Input/IMC_Main.IMC_Main" 0 (struct))
  (`WidgetBlueprintLibrary.SetInputMode_GameOnly` self)
  (bind _asbp_hud_gp (cast `/Game/Assets/BP/BP_HUD_GP` (`self.GetHUD`)))
  (set `self.HUDRef` _asbp_hud_gp))

(event `EnhancedInput|/Game/Assets/BP/Input/IA_Pause`
  (params (ActionValue :type Boolean) (ElapsedSeconds :type "Float (double-precision)") (TriggeredSeconds :type "Float (double-precision)") (InputAction :type "InputAction Object Reference" :default "/Game/Assets/BP/Input/IA_Pause.IA_Pause"))
  (:`Completed`
    (`self.Toggle Pause`)))

(event `Toggle Pause`
  (bind _returnvalue (`GameplayStatics.GetPlayerController` 0))
  (bind _pauseref (`/Game/Assets/BP/BP_HUD_GP.PauseRef` (`self.HUDRef`)))
  (bind _isa (`/Engine/EditorBlueprintResources/StandardMacros.FlipFlop`)
    (:`A`
      _)
    (:`B`
      _))
  (`GameplayStatics.SetGamePaused` _isa)
  (set `self.bShowMouseCursor` _isa)
  (if _isa
    (`Widget.SetVisibility` _pauseref "Visible")
    (`WidgetBlueprintLibrary.SetInputMode_GameAndUIEx` _returnvalue _pauseref)
    (message `/Game/Assets/BP/BPI_HUDUpdates.UpdateObjectiveText` (`self.GetHUD`) "" 5.0)
    (else
      (`Widget.SetVisibility` _pauseref "Collapsed")
      (`WidgetBlueprintLibrary.SetInputMode_GameOnly` _returnvalue))))

(fn `UserConstructionScript`)