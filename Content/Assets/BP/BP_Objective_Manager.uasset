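; Objective manager that counts destroyed quest actors toward a total taken from the QuestActors list at BeginPlay.
; UpdateQuest increments the count and, when it equals the total, CompletedQuest calls Activate on every ActivatedTargets entry.
; The loop binding UpdateQuest to each actor's OnDestroyed is disconnected, so this graph never registers it.
; A separate UpdateHUD function, uncalled here, sends remaining/total objective text to the player's HUD.
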(event `self.ReceiveBeginPlay`
  ; Initialize Quest
  (set `self.TotalObjectiveCount` (`KismetArrayLibrary.Array_Length` (`self.QuestActors`))))

(event `UpdateQuest` :!signature `self.OnDestroyed`
  (params (DestroyedActor :type "Actor Object Reference"))
  ; Update Quest
  (bind _result (`/Engine/EditorBlueprintResources/StandardMacros.IncrementInt` (`self.CurrentObjectiveCount`))
    (:`  `
      (if (== (`self.TotalObjectiveCount`) _result)
        (`self.CompletedQuest`)))))

(event `CompletedQuest`
  ; Complete Quest
  (for _array_element (`self.ActivatedTargets`)
    (`/Game/Assets/BP/BP_Activated_Actor.Activate` _array_element)))

(fn `UpdateHUD`
  (bind _totalobjectivecount (`self.TotalObjectiveCount`))
  (message `/Game/Assets/BP/BPI_HUDUpdates.UpdateObjectiveText` (`PlayerController.GetHUD` (`GameplayStatics.GetPlayerController` 0)) (`|FormatText` "{Object Type} {Current}/{Total}" _ (- _totalobjectivecount (`self.CurrentObjectiveCount`)) _totalobjectivecount) 3.0))

(fn `UserConstructionScript`)