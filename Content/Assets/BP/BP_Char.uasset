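; BP_Char is a player character Blueprint that handles basic movement, jumping and camera look through Enhanced Input actions.
; Locomotion and strafing inputs add movement along the actor's forward and right vectors, while horizontal and vertical look inputs drive controller yaw and pitch.
; Jump fires when its action starts; the primary action event is an empty placeholder, and the construction script does nothing.
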(event `EnhancedInput|/Game/Assets/BP/Input/IA_Primary`
  (params (ActionValue :type Boolean) (ElapsedSeconds :type "Float (double-precision)") (TriggeredSeconds :type "Float (double-precision)") (InputAction :type "InputAction Object Reference" :default "/Game/Assets/BP/Input/IA_Primary.IA_Primary"))
  ; Mechanics
)

(event `EnhancedInput|/Game/Assets/BP/Input/IA_Jump`
  (params (ActionValue :type Boolean) (ElapsedSeconds :type "Float (double-precision)") (TriggeredSeconds :type "Float (double-precision)") (InputAction :type "InputAction Object Reference" :default "/Game/Assets/BP/Input/IA_Jump.IA_Jump"))
  ; Mechanics
  (:`Started`
    (`self.Jump`)))

(event `EnhancedInput|/Game/Assets/BP/Input/IA_Locomotion`
  (params (ActionValue :type "Float (double-precision)") (ElapsedSeconds :type "Float (double-precision)") (TriggeredSeconds :type "Float (double-precision)") (InputAction :type "InputAction Object Reference" :default "/Game/Assets/BP/Input/IA_Locomotion.IA_Locomotion"))
  ; Basic Movement
  (:`Triggered`
    (`self.AddMovementInput` (`self.GetActorForwardVector`) ActionValue)))

(event `EnhancedInput|/Game/Assets/BP/Input/IA_Strafing`
  (params (ActionValue :type "Float (double-precision)") (ElapsedSeconds :type "Float (double-precision)") (TriggeredSeconds :type "Float (double-precision)") (InputAction :type "InputAction Object Reference" :default "/Game/Assets/BP/Input/IA_Strafing.IA_Strafing"))
  ; Basic Movement
  (:`Triggered`
    (`self.AddMovementInput` (`self.GetActorRightVector`) ActionValue)))

(event `EnhancedInput|/Game/Assets/BP/Input/IA_LookH`
  (params (ActionValue :type "Float (double-precision)") (ElapsedSeconds :type "Float (double-precision)") (TriggeredSeconds :type "Float (double-precision)") (InputAction :type "InputAction Object Reference" :default "/Game/Assets/BP/Input/IA_LookH.IA_LookH"))
  ; Camera Looking
  (:`Triggered`
    (`self.AddControllerYawInput` ActionValue)))

(event `EnhancedInput|/Game/Assets/BP/Input/IA_LookV`
  (params (ActionValue :type "Float (double-precision)") (ElapsedSeconds :type "Float (double-precision)") (TriggeredSeconds :type "Float (double-precision)") (InputAction :type "InputAction Object Reference" :default "/Game/Assets/BP/Input/IA_LookV.IA_LookV"))
  ; Camera Looking
  (:`Triggered`
    (`self.AddControllerPitchInput` ActionValue)))

(fn `UserConstructionScript`)