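; BP_HUD_GP sets up the player's gameplay HUD and pause screen widgets and relays objective text updates.
; On BeginPlay it creates WBP_PauseScreen, which starts collapsed, and WBP_HUD for player controller 0, adds both to the player screen and keeps references to them.
; The UpdateObjectiveText event forwards text and duration to the HUD widget.
; An unconnected node to collapse the HUD never runs.
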(event `self.ReceiveBeginPlay`
  (bind _returnvalue (`GameplayStatics.GetPlayerController` 0))
  (`|ExecutionSequence`
    (:`then_0`
      (bind _returnvalue_2 (`|CreateWidget` "/Game/Assets/UI/WBP_PauseScreen.WBP_PauseScreen_C" _returnvalue))
      (bind _output_get (set `self.PauseRef` _returnvalue_2))
      (`UserWidget.AddToPlayerScreen` _output_get 0)
      (`Widget.SetVisibility` _output_get "Collapsed"))
    (:`then_1`
      (bind _returnvalue_3 (`|CreateWidget` "/Game/Assets/UI/WBP_HUD.WBP_HUD_C" _returnvalue))
      (bind _output_get_2 (set `self.HUDRef` _returnvalue_3))
      (`UserWidget.AddToPlayerScreen` _output_get_2 0))))

(event `/Game/Assets/BP/BPI_HUDUpdates.UpdateObjectiveText`
  (params (Objective_Text :type Text) (Duration :type "Float (double-precision)"))
  (`/Game/Assets/UI/WBP_HUD.UpdateObjective` (`self.HUDRef`) Duration Objective_Text))

(fn `UserConstructionScript`)