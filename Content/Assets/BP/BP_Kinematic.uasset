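; BP_Kinematic is a moving object that the player character activates, gated by a lockable component.
; Hitting the Cube plays a timeline, or entering the Trigger does when UseTrigger is set; leaving the Trigger always reverses it.
; Each timeline update moves Pivot by interpolating between Start and End transforms if BPCLockable is unlocked, otherwise shows a "Locked" HUD message.
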(event `self.Cube.OnComponentHit`
  (params (HitComponent :type "PrimitiveComponent Object Reference") (OtherActor :type "Actor Object Reference") (OtherComp :type "PrimitiveComponent Object Reference") (NormalImpulse :type "Vector Structure") (Hit :type "HitResult Structure (by ref)"))
  (cast `/Game/Assets/BP/BP_Char` OtherActor)
  (if (not (`self.UseTrigger`))
    (bind (_direction _alpha) (`Timeline|Kinematic Timeline` :!label _label)
      (:`Update`
        (if (`/Game/Assets/BP/BPC_Lockable.Unlocked` (`self.BPC_Lockable`))
          (`SceneComponent.K2_SetWorldTransform` (`self.Pivot`) (`KismetMathLibrary.TLerp` (`SceneComponent.K2_GetComponentToWorld` (`self.Start`)) (`SceneComponent.K2_GetComponentToWorld` (`self.End`)) _alpha) false false)
          (else
            (message `/Game/Assets/BP/BPI_HUDUpdates.UpdateObjectiveText` (`PlayerController.GetHUD` (`GameplayStatics.GetPlayerController` 0)) "Locked" 3.0)))))))

(event `self.Trigger.OnComponentBeginOverlap`
  (params (OverlappedComponent :type "PrimitiveComponent Object Reference") (OtherActor :type "Actor Object Reference") (OtherComp :type "PrimitiveComponent Object Reference") (OtherBodyIndex :type Integer) (bFromSweep :type Boolean) (SweepResult :type "HitResult Structure (by ref)"))
  (cast `/Game/Assets/BP/BP_Char` OtherActor)
  (if (`self.UseTrigger`)
    (goto _label)))

(event `self.Trigger.OnComponentEndOverlap`
  (params (OverlappedComponent :type "PrimitiveComponent Object Reference") (OtherActor :type "Actor Object Reference") (OtherComp :type "PrimitiveComponent Object Reference") (OtherBodyIndex :type Integer))
  (cast `/Game/Assets/BP/BP_Char` OtherActor)
  (if (`self.UseTrigger`)
    (goto _label :!via `Reverse`)))

(fn `UserConstructionScript`)